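; Beauty-shot character Blueprint for the modular Survival female hero, with switchable views.
; The construction script binds body, clothing, headgear, prop and weapon components to the main Mesh as master pose, so they share its animation.
; The View input flip-flops which of V1 and V2 is active, enabling controller yaw rotation in both states.
; Tab opens the MVV level.
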(event Collision|EventActorBeginOverlap
  (params (OtherActor :type Actor%20Object%20Reference)))

(event EventTick
  (params (DeltaSeconds :type Float%20%28single-precision%29)))

(event Input|ActionEvents|InputActionView
  (params (Key :type Key%20Structure :default "None"))
  (:Pressed
    (Utilities|FlowControl|FlipFlop
      (:A
        (Components|Activation|SetActive (Variables|Default|GetV1) true false)
        (Components|Activation|SetActive (Variables|Default|GetV2) false false)
        (Variables|Default|SetbUseControllerRotationYaw true))
      (:B
        (Components|Activation|SetActive (Variables|Default|GetV1) false false)
        (Components|Activation|SetActive (Variables|Default|GetV2) true false)
        (Variables|Default|SetbUseControllerRotationYaw true)))))

(event Input|KeyboardEvents|Tab
  (params (Key :type Key%20Structure :default "None"))
  (:Pressed
    (Game|OpenLevel(byName) "MVV")))

(fn ConstructionScript
  (Class|SkinnedMeshComponent|SetMasterPoseComponent (Variables|Default|GetBody%20Part%2002) (Variables|Character|GetMesh) false))